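; BP_Torch is a torch actor with a point light and fire particle system whose color varies with game state.
; The construction script turns the light and fire blue when the IsGoal flag is set.
; On BeginPlay, it turns both red in the "End" level if the game instance's IsClear flag is false.
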(event `self.ReceiveBeginPlay`
  (bind _returnvalue (`GameplayStatics.GetCurrentLevelName` true))
  (if (and (`KismetStringLibrary.EqualEqual_StrStr` _returnvalue "End") (not (`/Game/BP/Award_GameInstans.IsClear` (cast `/Game/BP/Award_GameInstans` (`GameplayStatics.GetGameInstance`) :!pure true))))
    (`LightComponent.SetLightColor` (`self.PointLight`) (struct :`R` 1.0 :`A` 1.0) true)
    (`ParticleSystemComponent.SetColorParameter` (`self.ParticleSystem`) "FireColor" (struct :`R` 1.0 :`A` 1.0))))

(fn `UserConstructionScript`
  (if (`self.isGoal`)
    (`LightComponent.SetLightColor` (`self.PointLight`) (struct :`R` 0.0079 :`B` 1.0 :`A` 1.0) true)
    (`ParticleSystemComponent.SetColorParameter` (`self.ParticleSystem`) "FireColor" (struct :`B` 1.0 :`A` 1.0))))