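; Game mode for the Award game that runs a play session across numbered floor stages.
; On BeginPlay it resets the game instance's run stats, streams in Floor1, creates the UI, shows a paused tutorial, starts a capped timer and plays BGM.
; A destroyed player pawn respawns at the player start, repossessed and rebound.
; NextStage derives the next level name by incrementing its number, swaps streamed levels and repositions the pawn.
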(event `self.ReceiveBeginPlay`
  ;[1 1 1] 初期化処理
  (`self.Initial Game instance`)
  (`self.RespawnEvent`)
  (`self.LoadStage`)
  (`self.CreateUI`)
  (`self.Tutorial`)
  (`self.Time`)
  (`GameplayStatics.PlaySound2D` "/Game/Audio/bgm.bgm"))

(event `RespawnEvent`
  ;[1 1 1] アワード君のスポーン関係
  (add `self.OnDestroyed` (`GameplayStatics.GetPlayerPawn` 0) (delegate `RespawnAward`)))

(event `Tutorial`
  ;[1 1 1] チュートリアル
  (bind _returnvalue (`|CreateWidget` "/Game/UI/W_Floor.W_Floor_C"))
  (`UserWidget.AddToViewport` _returnvalue 0)
  (`GameplayStatics.SetGamePaused` true))

(event `RespawnAward` :!signature `self.OnDestroyed`
  (params (DestroyedActor :type "Actor Object Reference"))
  (bind _returnvalue (`GameplayStatics.GetPlayerController` 0))
  ;[1 1 1] アワード君のスポーン関係
  (bind _returnvalue_2 (`|SpawnActorFromClass` "/Game/BP/BPAward.BPAward_C" (`self.GetTransform` (`self.K2_FindPlayerStart` null)) "Undefined" "OverrideRootScale" null null))
  (`Controller.Possess` _returnvalue _returnvalue_2)
  (`PlayerController.SetAudioListenerOverride` :`self` _returnvalue :`AttachToComponent` (`/Game/BP/BPAward.PointLight` _returnvalue_2))
  (`self.RespawnEvent`))

(event `LoadStage`
  ;[1 1 1] ステージの読み込み
  (`GameplayStatics.LoadStreamLevel` (`/Game/BP/Award_GameInstans.Stage` (`self.AGIar`)) true true)
  (`self.Set Award Transform`))

(event `CreateUI`
  ;[1 1 1] UI関係
  (`|ExecutionSequence`
    (:`then_0`
      (bind _returnvalue (`|CreateWidget` "/Game/UI/W_Play.W_Play_C"))
      (`UserWidget.AddToViewport` _returnvalue 0))
    (:`then_1`
      (bind (_dulaytion _returnvalue_2) (`/Game/BP/Award_GameInstans.Loading` (`self.AGIar`)))
      (bind _output_get (set `self.LoadingWidget` _returnvalue_2))
      (`Widget.SetVisibility` _output_get "Hidden"))))

(event `NextStage`
  (bind _agiar (`self.AGIar`))
  (bind _stage (`/Game/BP/Award_GameInstans.Stage` _agiar))
  (bind _returnvalue (`KismetStringLibrary.Conv_NameToString` _stage))
  ;[1 1 1] ステージ遷移関係
  (`GameplayStatics.UnloadStreamLevel` _stage)
  (bind _output_get (set `/Game/BP/Award_GameInstans.Stage` (`KismetStringLibrary.Conv_StringToName` (`KismetStringLibrary.Concat_StrStr` (`KismetStringLibrary.Left` _returnvalue 5) (`KismetStringLibrary.Conv_IntToString` (+ (`KismetStringLibrary.Conv_StringToInt` (`KismetStringLibrary.RightChop` _returnvalue 5)) 1)))) _agiar))
  (`GameplayStatics.LoadStreamLevel` _output_get true true)
  (`self.Set Award Transform`))

(event `Initial Game instance`
  (bind _asaward_game_instans (cast `/Game/BP/Award_GameInstans` (`GameplayStatics.GetGameInstance`) :!pure true))
  ;[1 1 1] リザルト
  (set `self.AGIar` _asaward_game_instans)
  (set `/Game/BP/Award_GameInstans.Life` 2 _asaward_game_instans)
  (set `/Game/BP/Award_GameInstans.IsClear` false _asaward_game_instans)
  (set `/Game/BP/Award_GameInstans.Item` 0 _asaward_game_instans)
  (set `/Game/BP/Award_GameInstans.Minite` 0 _asaward_game_instans)
  (set `/Game/BP/Award_GameInstans.Second` 0 _asaward_game_instans)
  (set `/Game/BP/Award_GameInstans.Stage` "Floor1" _asaward_game_instans))

(event `Time`
  ;[1 1 1] 時間関係
  (`KismetSystemLibrary.K2_SetTimerDelegate` (delegate `Count UP`) 1.0 true))

(event `Count UP`
  (bind _agiar (`self.AGIar`))
  (bind _second (`/Game/BP/Award_GameInstans.Second` _agiar))
  ;[1 1 1] 時間関係
  (if (not (and (== (`/Game/BP/Award_GameInstans.Minite` _agiar) 99) (== (`/Game/BP/Award_GameInstans.Second` _agiar) 59)))
    (set `/Game/BP/Award_GameInstans.Second` (+ _second 1) _agiar)
    (if (> _second 59)
      (set `/Game/BP/Award_GameInstans.Minite` (+ (`/Game/BP/Award_GameInstans.Minite` _agiar) 1) _agiar)
      (set `/Game/BP/Award_GameInstans.Second` 0 _agiar))))

(fn `Set Award Transform`
  (`self.K2_SetActorTransform` (`GameplayStatics.GetPlayerPawn` 0) (`self.GetTransform` (`self.K2_FindPlayerStart` null)) false false))

(fn `UserConstructionScript`)