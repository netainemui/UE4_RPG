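; Player controller that moves its pawn a fixed distance along world X or Y for each W, A, S or D press.
; Each press records the start coordinate and sets a direction in Count, then Tick feeds movement input until MovingDistance is covered and idles Count at 99.
; Only forward checks MOVE and resets rotation to zero.
; Axis-based movement and a looped offset nudge are left disconnected.
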(event `self.ReceiveBeginPlay`)

(event `InputAxis|MoveForward`
  (params (AxisValue :type "Float (single-precision)")))

(event `InputAxis|MoveRight`
  (params (AxisValue :type "Float (single-precision)")))

(event `self.ReceiveTick`
  (params (DeltaSeconds :type "Float (single-precision)"))
  (bind _returnvalue (`self.K2_GetPawn`))
  (bind _returnvalue_x (`KismetMathLibrary.BreakVector` (`self.K2_GetActorLocation` (`self.K2_GetPawn`))))
  (bind (_returnvalue_x_2 _returnvalue_y) (`KismetMathLibrary.BreakVector` (`self.K2_GetActorLocation` (`self.K2_GetPawn`))))
  (bind _returnvalue_x_3 (`KismetMathLibrary.BreakVector` (`self.K2_GetActorLocation` (`self.K2_GetPawn`))))
  (bind (_returnvalue_x_4 _returnvalue_y_2) (`KismetMathLibrary.BreakVector` (`self.K2_GetActorLocation` (`self.K2_GetPawn`))))
  (switch `int` (`self.Count`)
    (:`0`
      (if (`self.MOVE`)
        (`self.K2_SetActorRotation` :`self` _returnvalue)
        (`Pawn.AddMovementInput` _returnvalue (1.0 0.0 0.0) 1.0 false)
        (if (>= _returnvalue_x_3 (+ (`self.StartPosition_X`) (`self.Moving distance`)))
          (set `self.Count` 99)
          (set `self.MOVE` false))
        (else
          (set `self.Count` 99))))
    (:`1`
      (`Pawn.AddMovementInput` (`self.K2_GetPawn`) (1.0 0.0 0.0) -1.0 false)
      (if (<= _returnvalue_x (- (`self.StartPosition_X`) (`self.Moving distance`)))
        (set `self.Count` 99)
        (set `self.MOVE` false)))
    (:`2`
      (`Pawn.AddMovementInput` (`self.K2_GetPawn`) (0.0 1.0 0.0) -1.0 false)
      (if (<= _returnvalue_y_2 (- (`self.StartPosition_Y`) (`self.Moving distance`)))
        (set `self.Count` 99)
        (set `self.MOVE` false)))
    (:`3`
      (`Pawn.AddMovementInput` (`self.K2_GetPawn`) (0.0 1.0 0.0) 1.0 false)
      (if (>= _returnvalue_y (+ (`self.StartPosition_Y`) (`self.Moving distance`)))
        (set `self.Count` 99)
        (set `self.MOVE` false)))))

(event `InputAction|Move_W`
  (params (Key :type "Key Structure"))
  (bind _returnvalue_x (`KismetMathLibrary.BreakVector` (`self.K2_GetActorLocation` (`self.K2_GetPawn`))))
  (:`Pressed`
    (set `self.StartPosition_X` _returnvalue_x)
    (set `self.Count` 0)
    (set `self.MOVE` true)))

(event `InputAction|Move_S`
  (params (Key :type "Key Structure"))
  (bind _returnvalue_x (`KismetMathLibrary.BreakVector` (`self.K2_GetActorLocation` (`self.K2_GetPawn`))))
  (:`Pressed`
    (set `self.StartPosition_X` _returnvalue_x)
    (set `self.Count` 1)
    (set `self.MOVE` true)))

(event `InputAction|Move_A`
  (params (Key :type "Key Structure"))
  (bind (_returnvalue_x _returnvalue_y) (`KismetMathLibrary.BreakVector` (`self.K2_GetActorLocation` (`self.K2_GetPawn`))))
  (:`Pressed`
    (set `self.StartPosition_Y` _returnvalue_y)
    (set `self.Count` 2)
    (set `self.MOVE` true)))

(event `InputAction|Move_D`
  (params (Key :type "Key Structure"))
  (bind (_returnvalue_x _returnvalue_y) (`KismetMathLibrary.BreakVector` (`self.K2_GetActorLocation` (`self.K2_GetPawn`))))
  (:`Pressed`
    (set `self.StartPosition_Y` _returnvalue_y)
    (set `self.Count` 3)
    (set `self.MOVE` true)))

(fn `UserConstructionScript`)